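; Player pawn Blueprint with test hooks for the Gameplay Ability System and montage root motion.
; After a short delay on BeginPlay, the server grants the GA_Test ability to the pawn's ability system component.
; Key 1 tries to activate GA_Test with remote activation allowed.
; Key 2 calls DisableRootMotionPredictedReplicated on the SGM montage component.
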(event `self.ReceiveBeginPlay`
  (bind _returnvalue (`AbilitySystemBlueprintLibrary.GetAbilitySystemComponent` null))
  (`KismetSystemLibrary.Delay` 0.2)
  (`/Engine/EditorBlueprintResources/ActorMacros.Switch Has Authority`
    (:`Authority`
      (`/Engine/EditorBlueprintResources/StandardMacros.IsValid` _returnvalue
        (:`Is Valid`
          (`AbilitySystemComponent.K2_GiveAbility` _returnvalue "/Game/Blueprint/GAS/GA_Test.GA_Test_C" 1 -1))))))

(event `Key|One`
  (params (Key :type "Key Structure"))
  (bind _returnvalue (`AbilitySystemBlueprintLibrary.GetAbilitySystemComponent` null))
  (:`Pressed`
    (`/Engine/EditorBlueprintResources/StandardMacros.IsValid` _returnvalue
      (:`Is Valid`
        (`AbilitySystemComponent.TryActivateAbilityByClass` _returnvalue "/Game/Blueprint/GAS/GA_Test.GA_Test_C" true)))))

(event `Key|Two`
  (params (Key :type "Key Structure"))
  (:`Pressed`
    (bind _sgm_montagecomponent (`self.SGM_MontageComponent`)
      (:`then`
        (`SGM_MontageComponent.DisableRootMotionPredictedReplicated` _sgm_montagecomponent))
      (:`else`))))

(fn `UserConstructionScript`)